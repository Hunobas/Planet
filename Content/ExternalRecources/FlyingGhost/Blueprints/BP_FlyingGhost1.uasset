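; BP_FlyingGhost1 is a flying ghost actor that moves by physics forces on its Cube component.
; Construction sets gravity, mass and targeting radius, and feeds eye location and glow color into the materials.
; AirMovement eases a locator's rotation toward a target, then pushes the Cube along a movement component's forward vector.
; The clamped force scales with distance beyond a standoff range, dropping to zero inside it.
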(fn `Air Movement`
  (params (`Target Loc` :type "Vector Structure") (`Movement Loc` :type "SceneComponent Object Reference") (Locator :type "SceneComponent Object Reference") (`Distance From Target` :type "Float (double-precision)") (Power :type "Float (double-precision)") (`Max Speed` :type "Float (double-precision)"))
  (bind _returnvalue (- `Target Loc` (`self.K2_GetActorLocation`)))
  (bind (_returnvalue_x _returnvalue_y _returnvalue_z) (`KismetMathLibrary.BreakVector` (* (`SceneComponent.GetForwardVector` `Movement Loc`) (`KismetMathLibrary.FClamp` (* (* (- (`KismetMathLibrary.VSize` _returnvalue) `Distance From Target`) Power 1.0) `Max Speed`) 0.0 50000.0))))
  (`SceneComponent.K2_SetRelativeRotation` Locator (`|EaseFunction` "EaseOut" (`self.Aiming Speed`) (`SceneComponent.RelativeRotation` Locator) (`KismetMathLibrary.MakeRotFromX` (`KismetMathLibrary.InverseTransformDirection` (`self.GetTransform`) _returnvalue)) true 1.0) false false)
  ;[0.7054 0.1159 0] Setting the direction and intensity of the force
  (`PrimitiveComponent.AddForceAtLocation` (`self.Cube`) (`KismetMathLibrary.MakeVector` _returnvalue_x _returnvalue_y (* _returnvalue_z 1.0)) (`SceneComponent.RelativeLocation` `Movement Loc`) "None"))

(fn `UserConstructionScript`
  (`PrimitiveComponent.SetEnableGravity` (`self.Cube`) (`self.Gravity`))
  (`PrimitiveComponent.SetMassOverrideInKg` (`self.Cube`) "None" (`self.Mass Scale`) true)
  (`MeshComponent.SetVectorParameterValueOnMaterials` (`self.Sphere1`) "Eye Location" (`SceneComponent.K2_GetComponentLocation` (`self.Eye`)))
  (`MeshComponent.SetVectorParameterValueOnMaterials` (`self.Eye`) "Glow Color" (`KismetMathLibrary.Conv_LinearColorToVector` (`self.Glow Color`)))
  (`MeshComponent.SetVectorParameterValueOnMaterials` (`self.Sphere1`) "Glow Color" (`KismetMathLibrary.Conv_LinearColorToVector` (`self.Glow Color`)))
  (`SphereComponent.SetSphereRadius` (`self.Targeting Range`) (`KismetMathLibrary.Conv_IntToDouble` (`self.Targeting Radius`)) true))