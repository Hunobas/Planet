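; Laser projectile from the Vefects Space VFX pack that homes in on an assigned Victim and triggers its shield hit.
; After a brief hidden delay on BeginPlay, it faces the Victim once, then moves toward the Victim's current location each Tick at constant speed.
; On overlapping the Victim, it passes the hit position to BP_TargetShip, swaps laser effects for impact VFX and sound, and destroys itself when that effect finishes.
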(event `self.ReceiveActorBeginOverlap`
  (params (OtherActor :type "Actor Object Reference"))
  (bind _ns_laser (`self.NS_Laser`))
  (bind _victim (`self.Victim`))
  (if (== OtherActor _victim)
    (bind _asbp_target_ship (cast `/Game/ExternalRecources/Vefects/Space_VFX/VFX/Blueprints/BP_TargetShip` _victim))
    (set `/Game/ExternalRecources/Vefects/Space_VFX/VFX/Blueprints/BP_TargetShip.ShieldHitPosition` (`SceneComponent.K2_GetComponentLocation` (`self.DefaultSceneRoot`)) _asbp_target_ship)
    (`/Game/ExternalRecources/Vefects/Space_VFX/VFX/Blueprints/BP_TargetShip.ShieldHit` _asbp_target_ship)
    (`ActorComponent.Deactivate` _ns_laser)
    (`ActorComponent.Deactivate` (`self.SFX_Missile_Loop`))
    (`SceneComponent.SetVisibility` _ns_laser false false)
    (`ActorComponent.Activate` (`self.NS_Impact`) false)
    (`GameplayStatics.PlaySoundAtLocation` "/Game/ExternalRecources/Vefects/Space_VFX/Audio/SFX_Vefects_Space_Laser_Impact_Cue.SFX_Vefects_Space_Laser_Impact_Cue" (`self.K2_GetActorLocation`) (struct) 1.0 1.0 0.0 null null null null)
    (add `NiagaraComponent.OnSystemFinished` (`self.NS_Impact`) (delegate `Impact_Finished`))))

(event `Impact_Finished`
  (params (PSystem :type "NiagaraComponent Object Reference"))
  (`self.K2_DestroyActor`))

(event `self.ReceiveTick`
  (params (DeltaSeconds :type "Float (single-precision)"))
  (if (`self.ShouldMove`)
    (bind _output_get (set `self.Speed` (`self.MaxSpeed`)))
    (`SceneComponent.K2_SetWorldLocation` (`self.DefaultSceneRoot`) (`KismetMathLibrary.VInterpTo_Constant` (`SceneComponent.K2_GetComponentLocation` (`self.DefaultSceneRoot`)) (`SceneComponent.K2_GetComponentLocation` (`Actor.RootComponent` (`self.Victim`))) DeltaSeconds (`KismetMathLibrary.FMin` _output_get (`self.MaxSpeed`))) false false)))

(event `self.ReceiveBeginPlay`
  (`SceneComponent.SetVisibility` (`self.NS_Laser`) false false)
  (`KismetSystemLibrary.Delay` 0.1)
  (`SceneComponent.K2_SetWorldRotation` (`self.DefaultSceneRoot`) (`KismetMathLibrary.Conv_VectorToRotator` (`KismetMathLibrary.Normal` (- (`self.K2_GetActorLocation` (`self.Victim`)) (`SceneComponent.K2_GetComponentLocation` (`self.DefaultSceneRoot`))))) false false)
  (set `self.ShouldMove` true)
  (`SceneComponent.SetVisibility` (`self.NS_Laser`) true false))

(fn `UserConstructionScript`)