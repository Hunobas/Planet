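; Attacking ship from the Vefects space VFX pack that repeatedly fires its selected Weapon at a Victim actor.
; BeginPlay loops Fire on FiringDelay, switching between missile types, a laser projectile and a hitscan beam; number keys also trigger most weapons.
; Projectiles spawn from a random left or right socket and receive the Victim.
; The beam line-traces from the center socket, sets Niagara beam and impact effects, and triggers BP_TargetShip's shield hit.
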(event `self.ReceiveBeginPlay`
  (`self.Fire` :!label _label)
  (`KismetSystemLibrary.Delay` (`self.FiringDelay`))
  (goto _label))

(event `Key|One`
  (params (Key :type "Key Structure"))
  (bind _staticmesh (`self.StaticMesh`))
  (:`Pressed`
    (if (`KismetMathLibrary.RandomBool`) :!label _label_2
      (bind _returnvalue (`|SpawnActorFromClass` "/Game/ExternalRecources/Vefects/Space_VFX/VFX/Blueprints/Missiles/BP_MissileExplosive.BP_MissileExplosive_C" (`SceneComponent.GetSocketTransform` _staticmesh "Weapon_Right" "RTS_World") "Undefined" "OverrideRootScale" null null))
      (set `/Game/ExternalRecources/Vefects/Space_VFX/VFX/Blueprints/Missiles/BP_MissileExplosive.Victim` (`self.Victim`) _returnvalue)
      (else
        (bind _returnvalue_2 (`|SpawnActorFromClass` "/Game/ExternalRecources/Vefects/Space_VFX/VFX/Blueprints/Missiles/BP_MissileExplosive.BP_MissileExplosive_C" (`SceneComponent.GetSocketTransform` _staticmesh "Weapon_Left" "RTS_World") "Undefined" "OverrideRootScale" null null))
        (set `/Game/ExternalRecources/Vefects/Space_VFX/VFX/Blueprints/Missiles/BP_MissileExplosive.Victim` (`self.Victim`) _returnvalue_2)))
    (`GameplayStatics.PlaySoundAtLocation` "/Game/ExternalRecources/Vefects/Space_VFX/Audio/SFX_Vefects_Space_Missile_Shot_Cue.SFX_Vefects_Space_Missile_Shot_Cue" (`self.K2_GetActorLocation`) (struct) 0.02 1.0 0.0 null null null null :!label _label_3)))

(event `Key|Three`
  (params (Key :type "Key Structure"))
  (bind _staticmesh (`self.StaticMesh`))
  (:`Pressed`
    (if (`KismetMathLibrary.RandomBool`) :!label _label_4
      (bind _returnvalue (`|SpawnActorFromClass` "/Game/ExternalRecources/Vefects/Space_VFX/VFX/Blueprints/Missiles/BP_MissileElectromagnetic.BP_MissileElectromagnetic_C" (`SceneComponent.GetSocketTransform` _staticmesh "Weapon_Right" "RTS_World") "Undefined" "OverrideRootScale" null null))
      (set `/Game/ExternalRecources/Vefects/Space_VFX/VFX/Blueprints/Missiles/BP_MissileElectromagnetic.Victim` (`self.Victim`) _returnvalue)
      (goto _label_3)
      (else
        (bind _returnvalue_2 (`|SpawnActorFromClass` "/Game/ExternalRecources/Vefects/Space_VFX/VFX/Blueprints/Missiles/BP_MissileElectromagnetic.BP_MissileElectromagnetic_C" (`SceneComponent.GetSocketTransform` _staticmesh "Weapon_Left" "RTS_World") "Undefined" "OverrideRootScale" null null))
        (set `/Game/ExternalRecources/Vefects/Space_VFX/VFX/Blueprints/Missiles/BP_MissileElectromagnetic.Victim` (`self.Victim`) _returnvalue_2)))))

(event `Fire`
  (bind _returnvalue (`self.K2_GetActorLocation`))
  (bind _staticmesh (`self.StaticMesh`))
  (bind _staticmesh_2 (`self.StaticMesh`))
  (bind _staticmesh_3 (`self.StaticMesh`))
  (bind _staticmesh_4 (`self.StaticMesh`))
  (bind _returnvalue_2 (`SceneComponent.GetSocketLocation` (`self.StaticMesh`) "Weapon_Center"))
  (switch `int` (`self.Weapon`)
    (:`0`
      (goto _label_2))
    (:`1`
      (goto _label_4))
    (:`2`
      (if (`KismetMathLibrary.RandomBool`) :!label _label_5
        (bind _returnvalue_3 (`|SpawnActorFromClass` "/Game/ExternalRecources/Vefects/Space_VFX/VFX/Blueprints/Missiles/BP_MissileKinetic.BP_MissileKinetic_C" (`SceneComponent.GetSocketTransform` _staticmesh_4 "Weapon_Right" "RTS_World") "Undefined" "OverrideRootScale" null null))
        (set `/Game/ExternalRecources/Vefects/Space_VFX/VFX/Blueprints/Missiles/BP_MissileKinetic.Victim` (`self.Victim`) _returnvalue_3)
        (goto _label_3)
        (else
          (bind _returnvalue_4 (`|SpawnActorFromClass` "/Game/ExternalRecources/Vefects/Space_VFX/VFX/Blueprints/Missiles/BP_MissileKinetic.BP_MissileKinetic_C" (`SceneComponent.GetSocketTransform` _staticmesh_4 "Weapon_Left" "RTS_World") "Undefined" "OverrideRootScale" null null))
          (set `/Game/ExternalRecources/Vefects/Space_VFX/VFX/Blueprints/Missiles/BP_MissileKinetic.Victim` (`self.Victim`) _returnvalue_4)
          (goto _label_3))))
    (:`3`
      (if (`KismetMathLibrary.RandomBool`) :!label _label_6
        (bind _returnvalue_5 (`|SpawnActorFromClass` "/Game/ExternalRecources/Vefects/Space_VFX/VFX/Blueprints/Missiles/BP_MissileBlackHole.BP_MissileBlackHole_C" (`SceneComponent.GetSocketTransform` _staticmesh_2 "Weapon_Right" "RTS_World") "Undefined" "OverrideRootScale" null null))
        (set `/Game/ExternalRecources/Vefects/Space_VFX/VFX/Blueprints/Missiles/BP_MissileBlackHole.Victim` (`self.Victim`) _returnvalue_5)
        (goto _label_3)
        (else
          (bind _returnvalue_6 (`|SpawnActorFromClass` "/Game/ExternalRecources/Vefects/Space_VFX/VFX/Blueprints/Missiles/BP_MissileBlackHole.BP_MissileBlackHole_C" (`SceneComponent.GetSocketTransform` _staticmesh_2 "Weapon_Left" "RTS_World") "Undefined" "OverrideRootScale" null null))
          (set `/Game/ExternalRecources/Vefects/Space_VFX/VFX/Blueprints/Missiles/BP_MissileBlackHole.Victim` (`self.Victim`) _returnvalue_6)
          (goto _label_3))))
    (:`4`
      (if (`KismetMathLibrary.RandomBool`) :!label _label_7
        (bind _returnvalue_7 (`|SpawnActorFromClass` "/Game/ExternalRecources/Vefects/Space_VFX/VFX/Blueprints/Missiles/BP_MissileWhiteHole.BP_MissileWhiteHole_C" (`SceneComponent.GetSocketTransform` _staticmesh_3 "Weapon_Right" "RTS_World") "Undefined" "OverrideRootScale" null null))
        (set `/Game/ExternalRecources/Vefects/Space_VFX/VFX/Blueprints/Missiles/BP_MissileWhiteHole.Victim` (`self.Victim`) _returnvalue_7)
        (goto _label_3)
        (else
          (bind _returnvalue_8 (`|SpawnActorFromClass` "/Game/ExternalRecources/Vefects/Space_VFX/VFX/Blueprints/Missiles/BP_MissileWhiteHole.BP_MissileWhiteHole_C" (`SceneComponent.GetSocketTransform` _staticmesh_3 "Weapon_Left" "RTS_World") "Undefined" "OverrideRootScale" null null))
          (set `/Game/ExternalRecources/Vefects/Space_VFX/VFX/Blueprints/Missiles/BP_MissileWhiteHole.Victim` (`self.Victim`) _returnvalue_8)
          (goto _label_3))))
    (:`5`
      ;[1 1 1] LASER
      (bind _returnvalue_9 (`NiagaraFunctionLibrary.SpawnSystemAtLocation` "/Game/ExternalRecources/Vefects/Space_VFX/VFX/Lasers/LongLaser/NS_Laser.NS_Laser" _returnvalue_2))
      (`GameplayStatics.PlaySoundAtLocation` "/Game/ExternalRecources/Vefects/Space_VFX/Audio/SFX_Vefects_Space_Laser_Shot_Cue.SFX_Vefects_Space_Laser_Shot_Cue" _returnvalue (struct) 0.2 1.0 0.0 null null null null)
      (bind (_outhit _returnvalue_10) (`KismetSystemLibrary.LineTraceSingle` _returnvalue_2 (`SceneComponent.K2_GetComponentLocation` (`Actor.RootComponent` (`self.Victim`))) "TraceTypeQuery1" false (`|MakeArray` self :!type "Actor Object Reference")))
      (if _returnvalue_10
        (`NiagaraComponent.SetVariableVec3` _returnvalue_9 "BeamEnd" (`.Location` (`GameplayStatics.BreakHitResult` _outhit)))
        (`NiagaraFunctionLibrary.SpawnSystemAtLocation` "/Game/ExternalRecources/Vefects/Space_VFX/VFX/Lasers/LongLaser/NS_LaserHit.NS_LaserHit" (`.Location` (`GameplayStatics.BreakHitResult` _outhit)) (`KismetMathLibrary.Conv_VectorToRotator` (`.ImpactNormal` (`GameplayStatics.BreakHitResult` _outhit))))
        (`GameplayStatics.PlaySoundAtLocation` "/Game/ExternalRecources/Vefects/Space_VFX/Audio/SFX_Vefects_Space_Laser_Impact_Cue.SFX_Vefects_Space_Laser_Impact_Cue" (`.Location` (`GameplayStatics.BreakHitResult` _outhit)) (struct) 1.0 1.0 0.0 null null null null)
        (bind _asbp_target_ship (cast `/Game/ExternalRecources/Vefects/Space_VFX/VFX/Blueprints/BP_TargetShip` (`self.Victim`)))
        (set `/Game/ExternalRecources/Vefects/Space_VFX/VFX/Blueprints/BP_TargetShip.ShieldHitPosition` (`.Location` (`GameplayStatics.BreakHitResult` _outhit)) _asbp_target_ship)
        (`/Game/ExternalRecources/Vefects/Space_VFX/VFX/Blueprints/BP_TargetShip.ShieldHit` _asbp_target_ship)))
    (:`6`
      (if (`KismetMathLibrary.RandomBool`) :!label _label_8
        (bind _returnvalue_11 (`|SpawnActorFromClass` "/Game/ExternalRecources/Vefects/Space_VFX/VFX/Blueprints/LaserProjectile/BP_LaserProjectile.BP_LaserProjectile_C" (`SceneComponent.GetSocketTransform` _staticmesh "Weapon_Right" "RTS_World") "Undefined" "OverrideRootScale" null null))
        (set `/Game/ExternalRecources/Vefects/Space_VFX/VFX/Blueprints/LaserProjectile/BP_LaserProjectile.Victim` (`self.Victim`) _returnvalue_11)
        (else
          (bind _returnvalue_12 (`|SpawnActorFromClass` "/Game/ExternalRecources/Vefects/Space_VFX/VFX/Blueprints/LaserProjectile/BP_LaserProjectile.BP_LaserProjectile_C" (`SceneComponent.GetSocketTransform` _staticmesh "Weapon_Left" "RTS_World") "Undefined" "OverrideRootScale" null null))
          (set `/Game/ExternalRecources/Vefects/Space_VFX/VFX/Blueprints/LaserProjectile/BP_LaserProjectile.Victim` (`self.Victim`) _returnvalue_12)))
      (`GameplayStatics.PlaySoundAtLocation` "/Game/ExternalRecources/Vefects/Space_VFX/Audio/SFX_Vefects_Space_Laser_Shot_Cue.SFX_Vefects_Space_Laser_Shot_Cue" _returnvalue (struct) 0.2 1.0 0.0 null null null null))))

(event `Key|Four`
  (params (Key :type "Key Structure"))
  (:`Pressed`
    (goto _label_5)))

(event `Key|Five`
  (params (Key :type "Key Structure"))
  (:`Pressed`
    (goto _label_6)))

(event `Key|Six`
  (params (Key :type "Key Structure"))
  (:`Pressed`
    (goto _label_7)))

(event `Key|Eight`
  (params (Key :type "Key Structure"))
  (:`Pressed`
    (goto _label_8)))

(fn `UserConstructionScript`)