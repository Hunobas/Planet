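; BP_Moon is a planetary environment Blueprint for a moon, with a StaticMesh and a Pivot component.
; Three timelines are set up to spin it a full turn: Rotate pitches both components, while the other two roll and yaw the Pivot respectively.
; None of the timelines is triggered, and BeginPlay and the construction script are empty, so this graph leaves the moon static.
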(event `self.ReceiveBeginPlay`)

(fn `UserConstructionScript`)