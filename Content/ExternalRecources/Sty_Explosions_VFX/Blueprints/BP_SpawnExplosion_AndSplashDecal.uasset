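; Actor that repeatedly spawns an explosion effect and explosion decal at its transform, with optional scattered splash decals.
; After a start delay it fires, then re-triggers itself indefinitely through a delayed Again event.
; Splash decals come from random line traces, starting ahead along the forward vector and cast back within a cone.
; Each hit spawns a short-lived splash decal aligned to the impact normal with random spin and size.
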(event `Again`
  (bind _returnvalue (`self.GetActorForwardVector`))
  (bind _location (.location (`self.GetTransform`)))
  (bind _returnvalue_2 (+ _location (* _returnvalue (* (`self.DecalSize`) 200.0))))
  (`KismetSystemLibrary.Delay` (`self.Delay`))
  (`NiagaraFunctionLibrary.SpawnSystemAtLocation` (`self.System Template`) _location (.rotation (`self.GetTransform`)) :!label _label)
  (`|SpawnActorFromClass` "/Game/ExternalRecources/Sty_Explosions_VFX/Blueprints/BP_ExplosionDecal.BP_ExplosionDecal_C" (`KismetMathLibrary.MakeTransform` _location (`KismetMathLibrary.MakeRotFromZ` (`self.GetActorForwardVector`)) (`KismetMathLibrary.MakeVector` 0.5 (.y (`KismetMathLibrary.Conv_DoubleToVector` (`self.DecalSize`))) (.z (`KismetMathLibrary.Conv_DoubleToVector` (`self.DecalSize`))))) "Undefined" "MultiplyWithRoot" null 0.0 1.0 2.0 (`self.Decal Material`) (`self.Emissive`) (`self.Emissive Duration`) 0.0 null)
  (`|ExecutionSequence`
    (:`then_0`
      (`self.Again`))
    (:`then_1`
      (if (`self.Splash`)
        (set `self.PoisonDecal` 0)
        (while (< (`self.PoisonDecal`) (`self.MaxPoisonDecal`))
          (`/Engine/EditorBlueprintResources/StandardMacros.IncrementInt` (`self.PoisonDecal`)
            (:`  `
              (bind (_outhit _returnvalue_3) (`KismetSystemLibrary.LineTraceSingle` _returnvalue_2 (+ _returnvalue_2 (* (`KismetMathLibrary.RandomUnitVectorInConeInDegrees` _returnvalue (`self.ConeAngle`)) -1000.0)) "TraceTypeQuery1"))
              (if _returnvalue_3
                (bind (_bblockinghit _binitialoverlap _time _distance _location_2 _impactpoint _normal _impactnormal) (`GameplayStatics.BreakHitResult` _outhit))
                (`|SpawnActorFromClass` "/Game/ExternalRecources/Sty_Explosions_VFX/Blueprints/BP_Splash_Decal.BP_Splash_Decal_C" (`KismetMathLibrary.MakeTransform` _impactpoint (`KismetMathLibrary.MakeRotFromZY` _impactnormal (`KismetMathLibrary.Cross_VectorVector` (`KismetMathLibrary.Normal` _impactnormal) (`KismetMathLibrary.RandomUnitVector`))) (`KismetMathLibrary.MakeVector` 0.1 (`KismetMathLibrary.RandomFloatInRange` 0.35 0.45) (`KismetMathLibrary.RandomFloatInRange` 0.35 0.45))) "Undefined" "MultiplyWithRoot" null 0.0 3.0 (`self.Splash_Decal_Material`) null)))))))))

(event `self.ReceiveBeginPlay`
  (`KismetSystemLibrary.Delay` (`self.StartDelay`))
  (goto _label))

(fn `UserConstructionScript`)