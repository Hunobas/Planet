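; BP_Heallvl3 is a level 3 heal area effect actor that periodically plays healing visuals on nearby tagged pawns.
; After an initial delay on BeginPlay, a self-recalling event repeatedly reactivates the HealLvl3 effect and sphere-traces for Pawn objects around the actor.
; Blocking hits on components tagged "Heal" get a P_Healcharacter effect spawned at their XY position and the actor's height.
; It applies no actual healing, only VFX.
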(event `Again`
  (bind (_returnvalue_x _returnvalue_y _returnvalue_z) (`KismetMathLibrary.BreakVector` (`self.K2_GetActorLocation`)))
  (`KismetSystemLibrary.Delay` 8.0)
  (`ActorComponent.Activate` (`self.HealLvl3`) true :!label _label)
  (bind _outhits (`KismetSystemLibrary.SphereTraceMultiForObjects` (+ (`self.K2_GetActorLocation`) (0.0 0.0 10.0)) (`self.K2_GetActorLocation`) 240.0 (`|MakeArray` "ObjectTypeQuery3" :!type "EObjectTypeQuery Enum")))
  (`|ExecutionSequence`
    (:`then_0`
      (`self.Again`))
    (:`then_1`
      (for _array_element _outhits
        (bind (_bblockinghit _binitialoverlap _time _distance _location _impactpoint _normal _impactnormal _physmat _hitactor _hitcomponent) (`GameplayStatics.BreakHitResult` _array_element))
        (if _bblockinghit
          (if (`ActorComponent.ComponentHasTag` _hitcomponent "Heal")
            (bind (_returnvalue_x_2 _returnvalue_y_2) (`KismetMathLibrary.BreakVector` (`SceneComponent.K2_GetComponentLocation` _hitcomponent)))
            (`NiagaraFunctionLibrary.SpawnSystemAtLocation` "/Game/ExternalRecources/Stylized_VFX_StPack/Particles/P_Healcharacter.P_Healcharacter" (`KismetMathLibrary.MakeVector` _returnvalue_x_2 _returnvalue_y_2 _returnvalue_z))))))))

(event `self.ReceiveBeginPlay`
  (`KismetSystemLibrary.Delay` 4.5)
  (goto _label))

(fn `UserConstructionScript`)