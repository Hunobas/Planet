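; Effect spawner that plays one of three StoneShield Niagara systems at the actor's location and rotation, chosen by its Level variable.
; BeginPlay delays the first spawn in proportion to Level, so the three variants start staggered.
; After each spawn the Again event calls itself and waits on a fixed delay before respawning the same variant, forming an endless loop.
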(event `Again`
  (bind _returnvalue (`self.K2_GetActorLocation`))
  (bind _returnvalue_2 (`self.K2_GetActorRotation`))
  (`KismetSystemLibrary.Delay` 12.0)
  (switch `int` (`self.Level`) :!label _label
    (:`1`
      (`NiagaraFunctionLibrary.SpawnSystemAtLocation` "/Game/ExternalRecources/Stylized_VFX_StPack/Particles/UPDATE_1_3/P_StoneShield_01.P_StoneShield_01" _returnvalue _returnvalue_2))
    (:`2`
      (`NiagaraFunctionLibrary.SpawnSystemAtLocation` "/Game/ExternalRecources/Stylized_VFX_StPack/Particles/UPDATE_1_3/P_StoneShield_02.P_StoneShield_02" _returnvalue _returnvalue_2))
    (:`3`
      (`NiagaraFunctionLibrary.SpawnSystemAtLocation` "/Game/ExternalRecources/Stylized_VFX_StPack/Particles/UPDATE_1_3/P_StoneShield_03.P_StoneShield_03" (`self.K2_GetActorLocation`) (`self.K2_GetActorRotation`))))
  (`self.Again`))

(event `self.ReceiveBeginPlay`
  (`KismetSystemLibrary.Delay` (- (* (`self.Level`) 4.0) 4.0))
  (goto _label))

(fn `UserConstructionScript`)