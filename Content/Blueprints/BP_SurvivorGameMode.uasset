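; Survivor game mode that drives enemy fire from MetaSound music cues.
; On BeginPlay it immediately adds a muted audio component and watches its "ClimateFixCue" output, with each change telling the FireManager to fire a random enemy.
; A second audio component, left unmuted, is added after the enemy fire delay plus a small offset, so the silent one runs ahead as a lookahead for the cues.
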(event `self.ReceiveBeginPlay`
  (`|ExecutionSequence`
    (:`then_0`
      (`KismetSystemLibrary.Delay` (+ (`self.EnemyFireDelay`) 0.25))
      (`AddComponent|NODE_AddAudioComponent-1`))
    (:`then_1`
      (bind _returnvalue (`AddComponent|NODE_AddAudioComponent-0`))
      (`MetaSoundOutputSubsystem.WatchOutput` (subsystem `MetaSoundOutputSubsystem`) _returnvalue "ClimateFixCue" (delegate `CueChange`) "None" "None")
      (`AudioComponent.SetVolumeMultiplier` _returnvalue 0.0))))

(event `CueChange`
  (params (OutputName :type Name) (Output :type "MetaSoundOutput Structure (by ref)"))
  (`EnemyFireManagerComponent.FireRandomEnemy` (`self.FireManager`)))

(fn `UserConstructionScript`)